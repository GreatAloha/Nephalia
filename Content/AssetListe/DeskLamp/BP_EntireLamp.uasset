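; BP_EntireLamp is an interactable desk lamp that the player switches on and off.
; Entering its trigger volume enables player input on the lamp, but only while the referenced Window reports closed; leaving the trigger disables it.
; The Interact input drives a FlipFlop that alternately activates and deactivates both lamp light components.
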(event `self.ReceiveBeginPlay`)

(event `self.ReceiveActorBeginOverlap`
  (params (OtherActor :type "Actor Object Reference")))

(event `self.ReceiveTick`
  (params (DeltaSeconds :type "Float (single-precision)")))

(event `self.Lamp_Trigger.OnComponentEndOverlap`
  (params (OtherActor :type "Actor Object Reference") (OtherComp :type "PrimitiveComponent Object Reference") (OtherBodyIndex :type Integer))
  (`self.DisableInput` (`GameplayStatics.GetPlayerController` 0)))

(event `self.Lamp_Trigger.OnComponentBeginOverlap`
  (params (OtherActor :type "Actor Object Reference") (OtherComp :type "PrimitiveComponent Object Reference") (OtherBodyIndex :type Integer) (bFromSweep :type Boolean) (SweepResult :type "HitResult Structure (by ref)"))
  (if (`/Game/AssetListe/Window/Window_TV.Window_Closed` (`self.Window`))
    (`self.EnableInput` (`GameplayStatics.GetPlayerController` 0))))

(event `InputAction|Interact`
  (params (Key :type "Key Structure" :default "AnyKey"))
  (:`Pressed`
    ;[1 1 1] Idea: Stands Right goes in and other way
    (`/Engine/EditorBlueprintResources/StandardMacros.FlipFlop`
      (:`A`
        (`ActorComponent.Activate` (`self.Lamp_Light1`) false)
        (`ActorComponent.Activate` (`self.Lamp_Light`) false))
      (:`B`
        (`ActorComponent.Deactivate` (`self.Lamp_Light1`))
        (`ActorComponent.Deactivate` (`self.Lamp_Light`))))))

(fn `UserConstructionScript`)