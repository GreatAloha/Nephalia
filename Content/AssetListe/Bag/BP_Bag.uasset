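; Bag actor with physgun-style pickup logic for the first-person character, built around a PhysGunPoint attached to the camera.
; Interact flip-flops: one press line-traces for a Puzzle_Piece, records it as held and snaps this actor's root to the point; the other has no effective release.
; DropObject and InterpolDistance handle release and smoothed hold distance, but nothing here calls them.
; BeginPlay uses the character reference before Interact assigns it.
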(event `self.ReceiveBeginPlay`)

(event `self.ReceiveActorBeginOverlap`
  (params (OtherActor :type "Actor Object Reference")))

(event `self.ReceiveTick`
  (params (DeltaSeconds :type "Float (single-precision)")))

(event `self.ReceiveBeginPlay`
  ;[1 1 1] Initialisation
  (bind _capsulecomponent (`Character.CapsuleComponent` (stale `InputAction|Interact` _asfirst_person_character)))
  (set `/Game/Standard_Blueprint/FirstPersonCharacter.CapsuleHalfHeight` (`CapsuleComponent.CapsuleHalfHeight` _capsulecomponent) (stale `InputAction|Interact` _asfirst_person_character))
  (set `/Game/Standard_Blueprint/FirstPersonCharacter.CapsuleRadius` (`CapsuleComponent.CapsuleRadius` _capsulecomponent) (stale `InputAction|Interact` _asfirst_person_character))
  (bind _firstpersoncamera (`/Game/Standard_Blueprint/FirstPersonCharacter.FirstPersonCamera` (stale `InputAction|Interact` _asfirst_person_character)))
  (`SceneComponent.K2_SetWorldLocation` (`/Game/Standard_Blueprint/FirstPersonCharacter.PhysGunPoint` (stale `InputAction|Interact` _asfirst_person_character)) (+ (`SceneComponent.K2_GetComponentLocation` _firstpersoncamera) (* (`KismetMathLibrary.GetForwardVector` (`KismetMathLibrary.MakeRotator` (.roll (`SceneComponent.K2_GetComponentRotation` _firstpersoncamera)) (.pitch (`SceneComponent.K2_GetComponentRotation` _firstpersoncamera)) (.yaw (`SceneComponent.K2_GetComponentRotation` _firstpersoncamera)))) (`self.PointDistance`))) false false)
  (`SceneComponent.K2_AttachTo` (`/Game/Standard_Blueprint/FirstPersonCharacter.PhysGunPoint` (stale `InputAction|Interact` _asfirst_person_character)) (`/Game/Standard_Blueprint/FirstPersonCharacter.FirstPersonCamera` (stale `InputAction|Interact` _asfirst_person_character)) "None" "KeepWorldPosition" true))

(event `DropObject`
  ;[1 1 1] Comment
  (bind _heldobjectpiece (`/Game/Standard_Blueprint/FirstPersonCharacter.HeldObjectPiece` (stale `InputAction|Interact` _asfirst_person_character)))
  (if (`KismetSystemLibrary.IsValid` _heldobjectpiece)
    (`self.DetachRootComponentFromParent` _heldobjectpiece true)
    (`PrimitiveComponent.SetSimulatePhysics` _heldobjectpiece true)
    (set `/Game/Standard_Blueprint/FirstPersonCharacter.HeldObjectPiece` null (stale `InputAction|Interact` _asfirst_person_character))))

(event `InputAction|Interact`
  (params (Key :type "Key Structure" :default "AnyKey"))
  ;[1 1 1] Trace and Snap Object to Actor
  (:`Pressed`
    (bind _asfirst_person_character (cast `/Game/Standard_Blueprint/FirstPersonCharacter` (stale `self.Trigger_Homework.OnComponentBeginOverlap` OtherActor)))
    (`/Engine/EditorBlueprintResources/StandardMacros.FlipFlop`
      (:`A`
        (set `/Game/Standard_Blueprint/FirstPersonCharacter.PhysGunDesiredDistance` (`/Game/Standard_Blueprint/FirstPersonCharacter.PointDistance` _asfirst_person_character) _asfirst_person_character)
        (set `/Game/Standard_Blueprint/FirstPersonCharacter.IsHoldingObject` false _asfirst_person_character)
        (bind _firstpersoncamera (`/Game/Standard_Blueprint/FirstPersonCharacter.FirstPersonCamera` _asfirst_person_character))
        (bind _returnvalue (`SceneComponent.K2_GetComponentLocation` _firstpersoncamera))
        (bind (_outhit _returnvalue_2) (`KismetSystemLibrary.LineTraceSingle` _returnvalue (+ _returnvalue (* (`KismetMathLibrary.GetForwardVector` (`KismetMathLibrary.MakeRotator` 0.0 (.pitch (`SceneComponent.K2_GetComponentRotation` _firstpersoncamera)) (.yaw (`SceneComponent.K2_GetComponentRotation` _firstpersoncamera)))) (`/Game/Standard_Blueprint/FirstPersonCharacter.GrabDistance` _asfirst_person_character))) "TraceTypeQuery1"))
        (if _returnvalue_2
          (bind (_bblockinghit _binitialoverlap _time _location _impactpoint _normal _impactnormal _physmat _hitactor) (`GameplayStatics.BreakHitResult` _outhit))
          (cast `Pawn` _hitactor
            (:`CastFailed`
              (bind _aspuzzle_piece (cast `/Game/GameplayElements/PianoPuzzle/Puzzle_Piece` _hitactor))
              (bind _output_get (set `/Game/Standard_Blueprint/FirstPersonCharacter.HeldObjectPiece` _aspuzzle_piece _asfirst_person_character))
              (if (`KismetSystemLibrary.IsValid` _output_get)
                (`self.K2_AttachRootComponentTo` (`/Game/Standard_Blueprint/FirstPersonCharacter.PhysGunPoint` _asfirst_person_character) "None" "SnapToTarget"))))))
      (:`B`
        (if (`/Game/Standard_Blueprint/FirstPersonCharacter.IsHoldingObject` _asfirst_person_character)
          (set `/Game/Standard_Blueprint/FirstPersonCharacter.IsHoldingObject` true _asfirst_person_character))))))

(event `self.Trigger_Homework.OnComponentBeginOverlap`
  (params (OtherActor :type "Actor Object Reference") (OtherComp :type "PrimitiveComponent Object Reference") (OtherBodyIndex :type Integer) (bFromSweep :type Boolean) (SweepResult :type "HitResult Structure (by ref)"))
  ;[1 1 1] Trace and Snap Object to Actor
)

(event `InterpolDistance`
  ;[1 1 1] Interpolate Between holding Distance
  (if (`/Game/Standard_Blueprint/FirstPersonCharacter.IsHoldingObject` (stale `InputAction|Interact` _asfirst_person_character))
    (if (`KismetSystemLibrary.IsValid` (`/Game/Standard_Blueprint/FirstPersonCharacter.HeldObjectPiece` (stale `InputAction|Interact` _asfirst_person_character)))
      (bind _physgundesireddistance (`/Game/Standard_Blueprint/FirstPersonCharacter.PhysGunDesiredDistance` (stale `InputAction|Interact` _asfirst_person_character)))
      (if (not (== (`self.PointDistance`) _physgundesireddistance))
        (set `self.PointDistance` (`KismetMathLibrary.FInterpTo` (`self.PointDistance`) _physgundesireddistance (`GameplayStatics.GetWorldDeltaSeconds`) 10.0))
        (bind _firstpersoncamera (`/Game/Standard_Blueprint/FirstPersonCharacter.FirstPersonCamera` (stale `InputAction|Interact` _asfirst_person_character)))
        (`SceneComponent.K2_SetWorldLocation` (`/Game/Standard_Blueprint/FirstPersonCharacter.PhysGunPoint` (stale `InputAction|Interact` _asfirst_person_character)) (+ (`SceneComponent.K2_GetComponentLocation` _firstpersoncamera) (* (`KismetMathLibrary.GetForwardVector` (`KismetMathLibrary.MakeRotator` 0.0 (.pitch (`SceneComponent.K2_GetComponentRotation` _firstpersoncamera)) (.yaw (`SceneComponent.K2_GetComponentRotation` _firstpersoncamera)))) (`self.PointDistance`))) false false)))))

(fn `UserConstructionScript`)