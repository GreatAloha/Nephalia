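; BP_ElevatorButton is an interactable elevator button that moves and flags itself as pressed.
; Overlapping the Open_Elevator component enables player input on the actor, and leaving it disables input.
; The first Interact press, gated by a never-reset DoOnce, plays a timeline that offsets the button along world X from its BeginPlay location and sets IsPressed.
; When the timeline finishes, IsPressed clears after a delay only if PersonalFile.PFRead is true.
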(event `self.ReceiveBeginPlay`)

(event `self.ReceiveActorBeginOverlap`
  (params (OtherActor :type "Actor Object Reference")))

(event `self.ReceiveTick`
  (params (DeltaSeconds :type "Float (single-precision)")))

(event `self.Open_Elevator.OnComponentEndOverlap`
  (params (OtherActor :type "Actor Object Reference") (OtherComp :type "PrimitiveComponent Object Reference") (OtherBodyIndex :type Integer))
  (`self.DisableInput` (`GameplayStatics.GetPlayerController` 0)))

(event `self.Open_Elevator.OnComponentBeginOverlap`
  (params (OtherActor :type "Actor Object Reference") (OtherComp :type "PrimitiveComponent Object Reference") (OtherBodyIndex :type Integer) (bFromSweep :type Boolean) (SweepResult :type "HitResult Structure (by ref)"))
  (`self.EnableInput` (`GameplayStatics.GetPlayerController` 0)))

(event `InputAction|Interact`
  (params (Key :type "Key Structure" :default "AnyKey"))
  (:`Pressed`
    (`/Engine/EditorBlueprintResources/StandardMacros.DoOnce` false
      (:`Completed`
        (bind (_direction _window) (`Timeline|Timeline_0`)
          (:`Update`
            (`SceneComponent.K2_SetWorldLocation` (`self.Elevator_Button`) (`KismetMathLibrary.MakeVector` (+ (.x (`self.Locator`)) _window) (.y (`self.Locator`)) (.z (`self.Locator`))) false false)
            (set `self.IsPressed` true))
          (:`Finished`
            (if (`/Game/AssetListe/Homework/PersonalFile.PFRead` (`self.PersonalFile`))
              (`KismetSystemLibrary.Delay` 8.0)
              (set `self.IsPressed` false))))))))

(event `self.ReceiveBeginPlay`
  (set `self.Locator` (`SceneComponent.K2_GetComponentLocation` (`self.Elevator_Button`))))

(fn `UserConstructionScript`)