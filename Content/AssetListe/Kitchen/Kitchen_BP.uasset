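; Interactive kitchen Blueprint where the player cooks a consumable on a heater and operates a sliding cabinet door.
; Overlap volumes toggle input based on inventory contents, with the pan volume also requiring a closed window.
; With FireON set, Interact lights the heater, removes consumables and runs a delayed pan, smoke and crispy-chicken sequence; switching off returns the food to inventory.
; A second Interact handler drives the door via timeline and sets PanTaken.
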(event `self.ReceiveActorBeginOverlap`
  (params (OtherActor :type "Actor Object Reference")))

(event `self.ReceiveTick`
  (params (DeltaSeconds :type "Float (single-precision)")))

(event `self.Fire_heater.OnComponentEndOverlap`
  (params (OtherActor :type "Actor Object Reference") (OtherComp :type "PrimitiveComponent Object Reference") (OtherBodyIndex :type Integer))
  (`self.DisableInput` (`GameplayStatics.GetPlayerController` 0)))

(event `self.Fire_heater.OnComponentBeginOverlap`
  (params (OtherActor :type "Actor Object Reference") (OtherComp :type "PrimitiveComponent Object Reference") (OtherBodyIndex :type Integer) (bFromSweep :type Boolean) (SweepResult :type "HitResult Structure (by ref)"))
  (bind _asfirst_person_character (cast `/Game/Standard_Blueprint/FirstPersonCharacter` OtherActor))
  (for _array_element (`/Game/Standard_Blueprint/FirstPersonCharacter.InventoryData` _asfirst_person_character)
    (if (`.IsTool_23_852F59F34A10BAE6BE8F20BA416EDFFF` (break `/Game/FirstPersonBP/Blueprints/ItemDataStructure` _array_element))
      (`self.EnableInput` (`GameplayStatics.GetPlayerController` 0)))))

(event `InputAction|Interact`
  (params (Key :type "Key Structure" :default "AnyKey"))
  (:`Pressed`
    ;[1 1 1] Idea: Stands Right goes in and other way
    (if (`self.HeaterStatus`)
      (set `self.HeaterStatus` false)
      (`ActorComponent.Deactivate` (`self.Fire`))
      ;[1 1 1] Comment
      (if (`self.MadeFood`)
        (set `self.CurrentItemID` (+ (`self.CurrentItemID`) 0.01))
        (bind _inventorydata (`/Game/Standard_Blueprint/FirstPersonCharacter.InventoryData` (stale _asfirst_person_character)))
        (bind (_name _thumbnail _isconsumable _itemid _weight _itemtextdata) (break `/Game/FirstPersonBP/Blueprints/ItemDataStructure` (stale _array_element)))
        (`KismetArrayLibrary.Array_Add` _inventorydata (make `/Game/FirstPersonBP/Blueprints/ItemDataStructure` _name _thumbnail _isconsumable (`self.CurrentItemID`) _weight _itemtextdata))
        (`ActorComponent.K2_DestroyComponent` (`self.Pan`))
        (`ActorComponent.K2_DestroyComponent` (`self.Chicken`))
        (`ActorComponent.Deactivate` (`self.Smoke`))
        (set `self.FoodEaten` true)
        (`AudioComponent.Stop` (`self.Pan_Sound`)))
      (elif (`/Game/Standard_Blueprint/FirstPersonCharacter.FireON` (`self.FPC`))
        (set `self.HeaterStatus` true)
        (`ActorComponent.Activate` (`self.Fire`) false)
        (bind _asfirst_person_character (cast `/Game/Standard_Blueprint/FirstPersonCharacter` (stale `self.Fire_heater.OnComponentBeginOverlap` OtherActor)))
        (for _array_element _inventorydata
          (if _isconsumable
            (`KismetArrayLibrary.Array_RemoveItem` _inventorydata _array_element)
            (`/Engine/EditorBlueprintResources/StandardMacros.DoOnce` false
              (:`Completed`
                (`SceneComponent.SetVisibility` (`self.Pan`) true false)
                (`SceneComponent.SetVisibility` (`self.Chicken`) true false)
                (`AudioComponent.Play` (`self.Pan_Sound`) 0.0)
                (`KismetSystemLibrary.Delay` 6.0)
                (`ActorComponent.SetActive` (`self.Smoke`) true false)
                (`PrimitiveComponent.SetMaterial` (`self.Chicken`) 0 "/Game/Materials/Experimental/Misc_Mat/Mat_Crispy.Mat_Crispy")
                (set `self.MadeFood` true)))))))))

(event `InputAction|Interact`
  (params (Key :type "Key Structure" :default "AnyKey"))
  (bind _close_wall (`self.Close_Wall`))
  ;[1 1 1] Comment
  (:`Pressed`
    (if (`self.IsOpen`)
      (`/Engine/EditorBlueprintResources/StandardMacros.DoOnce` false
        (:`Completed`
          (set `self.IsOpen` false)
          (`AudioComponent.Play` _close_wall 0.0)
          (bind (_direction _window) (`Timeline|Timeline_0` :!via `Reverse` :!label _label)
            (:`Update`
              (`SceneComponent.K2_SetWorldLocation` (`self.Kitchen_WashDoor_L2Open`) (`KismetMathLibrary.MakeVector` (- (.x (`self.Locator`)) _window) (.y (`self.Locator`)) (.z (`self.Locator`))) false false)
              (set `self.PanTaken` true)))))
      (else
        (`/Engine/EditorBlueprintResources/StandardMacros.DoOnce` false
          (:`Completed`
            (set `self.IsOpen` true)
            (`AudioComponent.Play` _close_wall 0.0)
            (goto _label)))))))

(event `self.ReceiveBeginPlay`
  (set `self.Locator` (`SceneComponent.K2_GetComponentLocation` (`self.Kitchen_WashDoor_L2Open`))))

(event `self.PickUp_Pan.OnComponentBeginOverlap`
  (params (OtherActor :type "Actor Object Reference") (OtherComp :type "PrimitiveComponent Object Reference") (OtherBodyIndex :type Integer) (bFromSweep :type Boolean) (SweepResult :type "HitResult Structure (by ref)"))
  ;[1 1 1] Comment
  (`self.DisableInput` (`GameplayStatics.GetPlayerController` 0)))

(event `self.PickUp_Pan.OnComponentEndOverlap`
  (params (OtherActor :type "Actor Object Reference") (OtherComp :type "PrimitiveComponent Object Reference") (OtherBodyIndex :type Integer))
  ;[1 1 1] Comment
  (if (`/Game/AssetListe/Window/Window_TV.Window_Closed` (`self.Window`))
    (bind _asfirst_person_character (cast `/Game/Standard_Blueprint/FirstPersonCharacter` OtherActor))
    (for _array_element (`/Game/Standard_Blueprint/FirstPersonCharacter.InventoryData` _asfirst_person_character)
      (if (`.IsConsumable_17_80979D5943DC60EEC636758303567A90` (break `/Game/FirstPersonBP/Blueprints/ItemDataStructure` _array_element))
        (`self.EnableInput` (`GameplayStatics.GetPlayerController` 0))))))

(fn `UserConstructionScript`)