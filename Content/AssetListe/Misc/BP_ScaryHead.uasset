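; BP_ScaryHead is a scary head pawn that chases the player once the phone has been answered.
; Both spotlights are hidden at BeginPlay.
; When PawnSensing sees the FirstPersonCharacter, it issues an AIMoveTo toward them.
; Right after issuing the move, without waiting for arrival, it sets Died if the character is not falling and its location matches the head's within a 300-unit tolerance.
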(event `self.ReceiveBeginPlay`
  (`SceneComponent.SetVisibility` (`self.SpotLight`) false false)
  (`SceneComponent.SetVisibility` (`self.SpotLight1`) false false))

(event `self.ReceiveActorBeginOverlap`
  (params (OtherActor :type "Actor Object Reference")))

(event `self.ReceiveTick`
  (params (DeltaSeconds :type "Float (single-precision)")))

(event `self.PawnSensing.OnSeePawn`
  (params (Pawn :type "Pawn Object Reference"))
  (if (`/Game/AssetListe/Phone/Act2_Phone.IsAnswered` (`self.Phone`))
    (bind _asfirst_person_character (cast `/Game/Standard_Blueprint/FirstPersonCharacter` Pawn))
    (`|AIMoveTo` self (0.0 0.0 0.0) _asfirst_person_character
      (:`then`
        (if (`NavMovementComponent.IsFalling` (`Character.CharacterMovement` _asfirst_person_character))
          _
          (elif (== (`self.K2_GetActorLocation` _asfirst_person_character) (`self.K2_GetActorLocation` self) :`ErrorTolerance` 300.0)
            (set `self.Died` true)))))))

(fn `UserConstructionScript`)